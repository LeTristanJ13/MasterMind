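; BP_Row is a clickable row of spheres for a Mastermind game.
; BeginPlay stores its four sphere references in Sphere0 through Sphere3.
; A click calls Clicked, then spawns the next BP_Row offset along world X with the same rotation and scale.
; It then calls Block on the MastermindSphere of each valid BP_Sphere in PlayerSpheres, stopping if a cast fails.
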(event `self.ReceiveBeginPlay`
  (set `self.Sphere_0` (`self.Sphere`))
  (set `self.Sphere_1` (`self.Sphere1`))
  (set `self.Sphere_2` (`self.Sphere2`))
  (set `self.Sphere_3` (`self.Sphere3`)))

(event `self.ReceiveTick`
  (params (DeltaSeconds :type "Float (single-precision)")))

(event `self.ReceiveActorOnClicked`
  (params (ButtonPressed :type "Key Structure"))
  (bind _returnvalue (`self.GetTransform`))
  (`self.Clicked`)
  (`|SpawnActorFromClass` "BP_Row_C" (`KismetMathLibrary.MakeTransform` (`KismetMathLibrary.MakeVector` (+ (.x (.location _returnvalue)) 200.0) (.y (.location _returnvalue)) (.z (.location _returnvalue))) (.rotation _returnvalue) (.scale _returnvalue)) "Undefined" "MultiplyWithRoot" null null)
  (for _array_element (`self.PlayerSpheres`)
    (`/Engine/EditorBlueprintResources/StandardMacros.IsValid` _array_element
      (:`Is Valid`
        (bind _asbp_sphere (cast `/Game/Mastermind/Blueprints/BP_Sphere` _array_element))
        (`MastermindSphere.Block` (`/Game/Mastermind/Blueprints/BP_Sphere.MastermindSphere` _asbp_sphere))))))

(fn `UserConstructionScript`)